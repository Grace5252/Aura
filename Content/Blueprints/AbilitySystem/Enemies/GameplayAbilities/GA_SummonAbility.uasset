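; Enemy summon ability, using the Shaman summon montage, that spawns random minions around its avatar.
; Shuffles the spawn locations, plays a ground effect at each, then waits for the montage's attack event.
; A short-delay loop then spawns one minion per location, raised by capsule half-height and facing outward, before ending the ability.
; Each spawn and later destruction updates the avatar's minion count.
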(event `self.K2_ActivateAbility`
  (bind _returnvalue (`self.GetSpawnLocations`))
  (bind _output_get (set `self.SpawnLocations` _returnvalue))
  (`KismetArrayLibrary.Array_Shuffle` _output_get)
  (for _array_element _output_get
    (`NiagaraFunctionLibrary.SpawnSystemAtLocation` "/Game/Assets/Effects/Combat/NS_GroundSummon.NS_GroundSummon" _array_element))
  (`AbilityTask_PlayMontageAndWait.CreatePlayMontageAndWaitProxy` "None" "/Game/Assets/Enemies/Shaman/Animations/AM_Shaman_Summon.AM_Shaman_Summon" 1.0 "None" false
    (:`then`
      (`AbilityTask_WaitGameplayEvent.WaitGameplayEvent` (struct :`TagName` "Montage.Attack.1") null true
        (:`EventReceived`
          (if (< (`self.SpawnLocationIndex`) (`KismetArrayLibrary.Array_Length` (`self.SpawnLocations`))) :!label _label
            (bind _spawned_actor (`self.SpawnMinion`))
            (add `Actor.OnDestroyed` _spawned_actor (delegate `OnDestroyed_Event`))
            (message `CombatInterface.AddToMinionCount` (`self.GetAvatarActorFromActorInfo`) 1)
            (`/Engine/EditorBlueprintResources/StandardMacros.IncrementInt` (`self.SpawnLocationIndex`)
              (:`  `
                (`KismetSystemLibrary.Delay` 0.2)
                (goto _label)))
            (else
              (`self.K2_EndAbility`))))))))

(event `OnDestroyed_Event`
  (params (DestroyedActor :type "Actor Object Reference"))
  (message `CombatInterface.AddToMinionCount` (`self.GetAvatarActorFromActorInfo`) -1))

(fn `SpawnMinion`
  (returns (`Spawned Actor` :type "AuraCharacterBase Object Reference"))
  (bind _returnvalue (`self.GetRandomMinionClass`))
  (bind _returnvalue_2 (`self.GetRandomMinionClassDefaultObject` _returnvalue))
  (bind _returnvalue_3 (+ (`|GetArrayItem` (`self.SpawnLocations`) (`self.SpawnLocationIndex`)) (`KismetMathLibrary.MakeVector` 0.0 0.0 (`CapsuleComponent.GetScaledCapsuleHalfHeight` (`Character.CapsuleComponent` _returnvalue_2)))))
  (bind _returnvalue_4 (`|SpawnActorFromClass` _returnvalue (`KismetMathLibrary.MakeTransform` _returnvalue_3 (`KismetMathLibrary.FindLookAtRotation` (`Actor.K2_GetActorLocation` (`self.GetAvatarActorFromActorInfo`)) _returnvalue_3)) "Undefined" "MultiplyWithRoot" null null))
  (return _returnvalue_4))