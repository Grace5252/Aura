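; Enemy melee attack gameplay ability that plays a random tagged attack montage from the avatar and damages nearby hostile players.
; A gameplay event matching the montage's tag triggers a radius query at the montage's combat socket, damaging living non-friendly players.
; Any hit fires one melee impact GameplayCue at the socket, carrying the montage tag and combat target.
; The ability ends after that check, when the montage finishes or is interrupted, or if no montage exists.
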(event `self.K2_ActivateAbility`
  (bind _returnvalue (`self.GetAvatarActorFromActorInfo`))
  (bind _returnvalue_2 (`self.GetAvatarActorFromActorInfo`))
  (set `self.HasHitTarget` false)
  (bind _returnvalue_3 (message `CombatInterface.GetAttackMontages` (`self.GetAvatarActorFromActorInfo`)))
  (bind (_outitem _outindex) (`KismetArrayLibrary.Array_Random` _returnvalue_3))
  (if (!= _outindex -1)
    (bind _output_get (set `self.TaggedMontage` _outitem))
    (bind (_montage _sockettag _montagetag) (break `TaggedMontage` _output_get))
    (set `self.SocketTag` _sockettag)
    (set `self.MontageTag` _montagetag)
    (`AbilityTask_PlayMontageAndWait.CreatePlayMontageAndWaitProxy` "None" _montage 1.0 "None" false
      (:`then`
        (`AbilityTask_WaitGameplayEvent.WaitGameplayEvent` (`self.MontageTag`) null
          (:`EventReceived`
            (bind _returnvalue_4 (message `CombatInterface.GetCombatSocketLocation` _returnvalue (`self.SocketTag`)))
            (bind _output_get_2 (set `self.CombatSocketLocation` _returnvalue_4))
            (bind _outoverlappingactors (`AuraAbilitySystemLibrary.GetLivePlayersWithinRadius` _returnvalue (`|MakeArray` _returnvalue) 200.0 _output_get_2))
            (for _array_element _outoverlappingactors
              (if (`AuraAbilitySystemLibrary.IsNotFriend` (`self.GetAvatarActorFromActorInfo`) _array_element)
                (`self.CauseDamage` _array_element)
                (set `self.HasHitTarget` true)))
            (if (`self.HasHitTarget`)
              (bind _returnvalue_5 (message `EnemyInterface.GetCombatTarget` _returnvalue_2))
              (`self.K2_ExecuteGameplayCueWithParams` (struct :`TagName` "GameplayCue.MeleeImpact") (`AbilitySystemBlueprintLibrary.MakeGameplayCueParameters` 0.0 0.0 (struct) (struct) (struct) (`BlueprintGameplayTagLibrary.MakeGameplayTagContainerFromTag` (`self.MontageTag`)) (struct) (`self.CombatSocketLocation`) (0.0 0.0 0.0) null _returnvalue_2 _returnvalue_5)))
            (`self.K2_EndAbility`))))
      (:`OnCompleted`
        (`self.K2_EndAbility` :!label _label))
      (:`OnInterrupted`
        (goto _label))
      (:`OnCancelled`
        (goto _label)))
    (else
      (`self.K2_EndAbility`))))

(event `self.K2_OnEndAbility`
  (params (bWasCancelled :type Boolean)))