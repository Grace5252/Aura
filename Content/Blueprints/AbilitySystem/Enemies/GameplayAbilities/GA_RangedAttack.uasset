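; Enemy gameplay ability that performs a ranged attack by firing a projectile at the avatar's combat target.
; It picks a random tagged montage through interface calls on the avatar and plays it, waiting for that montage's gameplay event.
; The event spawns the projectile from the montage's socket tag toward the target's location, then ends the ability while the montage keeps playing.
; It also ends if no montage exists or playback completes, is interrupted or cancelled.
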(event `self.K2_ActivateAbility`
  (bind _returnvalue (`self.GetAvatarActorFromActorInfo`))
  (bind _returnvalue_2 (message `CombatInterface.GetAttackMontages` (`self.GetAvatarActorFromActorInfo`)))
  (bind (_outitem _outindex) (`KismetArrayLibrary.Array_Random` _returnvalue_2))
  (if (!= _outindex -1)
    (bind _output_get (set `self.TaggedMontage` _outitem))
    (bind (_montage _sockettag _montagetag) (break `TaggedMontage` _output_get))
    (`AbilityTask_PlayMontageAndWait.CreatePlayMontageAndWaitProxy` "None" _montage 1.0 "None" false
      (:`then`
        (`AbilityTask_WaitGameplayEvent.WaitGameplayEvent` _montagetag null true
          (:`EventReceived`
            (message `CombatInterface.GetCombatSocketLocation` _returnvalue _sockettag)
            (bind _returnvalue_3 (message `EnemyInterface.GetCombatTarget` _returnvalue))
            (`self.SpawnProjectile` (`Actor.K2_GetActorLocation` _returnvalue_3) _sockettag)
            (`self.K2_EndAbility`))))
      (:`OnCompleted`
        (`self.K2_EndAbility` :!label _label))
      (:`OnInterrupted`
        (goto _label))
      (:`OnCancelled`
        (goto _label)))
    (else
      (`self.K2_EndAbility`))))