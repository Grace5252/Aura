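; Melee attack gameplay ability that plays a goblin spear attack montage and detects players hit by the strike.
; On activation it stores the avatar's combat target, then waits for the montage's attack gameplay event to query live players around the combat socket, ignoring the avatar.
; Found players currently get only debug spheres, with no damage applied.
; The ability ends when the montage completes, is interrupted or is cancelled.
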(event `self.K2_ActivateAbility`
  (bind _returnvalue (`self.GetAvatarActorFromActorInfo`))
  (bind _returnvalue_2 (message `EnemyInterface.GetCombatTarget` (`self.GetAvatarActorFromActorInfo`)))
  (set `self.CombatTarget` _returnvalue_2)
  (`AbilityTask_PlayMontageAndWait.CreatePlayMontageAndWaitProxy` "None" "/Game/Assets/Enemies/Goblin/Animations/Spear/AM_Attack_Goblin_Spear.AM_Attack_Goblin_Spear"
    (:`then`
      (`AbilityTask_WaitGameplayEvent.WaitGameplayEvent` (struct :`TagName` "Event.Montage.Attack") null
        (:`EventReceived`
          (bind _returnvalue_3 (message `CombatInterface.GetCombatSocketLocation` _returnvalue))
          (bind _outoverlappingactors (`AuraAbilitySystemLibrary.GetLivePlayersWithinRadius` _returnvalue (`|MakeArray` _returnvalue) 200.0 _returnvalue_3))
          (for _array_element _outoverlappingactors
            (`KismetSystemLibrary.DrawDebugSphere` (`Actor.K2_GetActorLocation` _array_element) 15.0 12 (struct :`R` 1.0 :`G` 0.314767 :`B` 0.235031 :`A` 1.0) 0.5 2.0)))))
    (:`OnCompleted`
      (`self.K2_EndAbility` :!label _label))
    (:`OnInterrupted`
      (goto _label))
    (:`OnCancelled`
      (goto _label))))

(event `self.K2_OnEndAbility`
  (params (bWasCancelled :type Boolean)))